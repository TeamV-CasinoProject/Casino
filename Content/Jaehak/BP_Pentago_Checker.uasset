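; BP_Pentago_Checker is a Pentago board checker that tracks a slot's stone state as a float SlotValue.
; BeginPlay clears the value and binds white and black spawn events, which set it to 1 or 2 respectively and print it.
; NewFunction, not called here, instead gives 1 for a black stone at the exact same location, 0 for one elsewhere, and 2 whenever the black-stone cast fails.
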(event Custom|SpawnWhite
  (bind _output_get (Variables|Default|Setslot_Value 1.0))
  (Development|PrintString (Utilities|String|ToString(Float) _output_get)))

(event Custom|SpawnBlack
  (bind _output_get (Variables|Default|Setslot_Value 2.0))
  (Development|PrintString (Utilities|String|ToString(Float) _output_get)))

(event EventBeginPlay
  (bind _self self)
  (bind _output_get (Variables|Default|Setslot_Value 0.0))
  (EventDispatchers|BindEventtoSpawnWhiteEvent _self (delegate Custom|SpawnWhite))
  (EventDispatchers|BindEventtoSpawnBlackEvent _self (delegate Custom|SpawnBlack)))

(fn ConstructionScript)

(fn NewFunction
  (params (SpawnActor :type Actor%20Object%20Reference))
  (Utilities|Casting|CastToBP_Pentago_Stone_Black SpawnActor
    (:then
      (if (Utilities|Operators|EqualEqual (Transformation|GetActorLocation SpawnActor) (Transformation|GetActorLocation self) 0.0)
        (Variables|Default|Setslot_Value 1.0)
        (else
          (Variables|Default|Setslot_Value 0.0 :!label _label))))
    (:CastFailed
      (if true
        (Variables|Default|Setslot_Value 2.0)
        (else
          (goto _label))))))