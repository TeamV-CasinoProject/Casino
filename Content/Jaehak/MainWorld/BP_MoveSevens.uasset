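; Interactable level-travel trigger (MoveSevens) that names a game on a prompt widget and sends the player to that game's level.
; BeginPlay writes GameName into the BP_Interaction_UI widget, and sphere overlap shows or hides it.
; Overlap start also binds PressedE, which after a short delay displays BP_LoadingWidget, waits, then opens the Level reference with DestinationTag as options.
; End overlap never unbinds PressedE.
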(event OnComponentBeginOverlap(Sphere)
  (params (OverlappedComponent :type Primitive%20Component%20Object%20Reference) (OtherActor :type Actor%20Object%20Reference) (OtherComp :type Primitive%20Component%20Object%20Reference) (OtherBodyIndex :type Integer) (bFromSweep :type Boolean) (SweepResult :type Hit%20Result%20Structure%20%28by%20ref%29))
  (Development|PrintString "StartOverlap")
  (Rendering|SetVisibility (Variables|Default|GetWidget) true false)
  (EventDispatchers|BindEventtoMoveSevens (delegate Custom|PressedE))
  (Development|PrintString "aaaaaaaaaaaaaaa"))

(event OnComponentEndOverlap(Sphere)
  (params (OverlappedComponent :type Primitive%20Component%20Object%20Reference) (OtherActor :type Actor%20Object%20Reference) (OtherComp :type Primitive%20Component%20Object%20Reference) (OtherBodyIndex :type Integer))
  (Development|PrintString "EndOverlap")
  (Rendering|SetVisibility (Variables|Default|GetWidget) false false))

(event Custom|PressedE
  (Development|PrintString "Pressed")
  (Utilities|FlowControl|Delay 1.0)
  (bind _returnvalue (Game|ConstructObjectfromClass "/Game/Jaehak/Widget/BP_LoadingWidget.BP_LoadingWidget_C"))
  (UserInterface|Viewport|AddtoViewport _returnvalue 0)
  (Utilities|FlowControl|Delay 3.0)
  (Game|OpenLevel(byObjectReference) (Variables|Default|GetLevel) true (Variables|Default|GetDestination%20Tag)))

(event EventBeginPlay
  (bind _asbp_interaction_ui (Utilities|Casting|CastToBP_Interaction_UI (UserInterface|GetUserWidgetObject (Variables|Default|GetWidget))))
  (Variables|/Game/Jaehak/Widget/BP_Interaction_UI.BP_Interaction_UI_C|SetNameValue _asbp_interaction_ui (Utilities|Text|ToText(String) (Variables|Default|GetGameName))))

(event Collision|EventActorBeginOverlap
  (params (OtherActor :type Actor%20Object%20Reference)))

(event EventTick
  (params (DeltaSeconds :type Float%20%28single-precision%29)))

(fn ConstructionScript)