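; Interactable portal actor that moves the player to another level, named for the blackjack game.
; A sphere overlap shows or hides an interaction widget labeled with the game name, and entering also binds the PressedE event.
; PressedE shows a loading widget between delays, stores a teleportation tag in the game instance and opens the level named by DestinationTag.
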(event OnComponentBeginOverlap(Sphere)
  (params (OverlappedComponent :type Primitive%20Component%20Object%20Reference) (OtherActor :type Actor%20Object%20Reference) (OtherComp :type Primitive%20Component%20Object%20Reference) (OtherBodyIndex :type Integer) (bFromSweep :type Boolean) (SweepResult :type Hit%20Result%20Structure%20%28by%20ref%29))
  (Rendering|SetVisibility (Variables|Default|GetWidget) true false)
  (EventDispatchers|BindEventtoMoveBlackJack (delegate Custom|PressedE)))

(event OnComponentEndOverlap(Sphere)
  (params (OverlappedComponent :type Primitive%20Component%20Object%20Reference) (OtherActor :type Actor%20Object%20Reference) (OtherComp :type Primitive%20Component%20Object%20Reference) (OtherBodyIndex :type Integer))
  (Rendering|SetVisibility (Variables|Default|GetWidget) false false))

(event Custom|PressedE
  (Utilities|FlowControl|Delay 1.0)
  (bind _returnvalue (Game|ConstructObjectfromClass "/Game/Jaehak/Widget/BP_LoadingWidget.BP_LoadingWidget_C"))
  (UserInterface|Viewport|AddtoViewport _returnvalue 0)
  (Utilities|FlowControl|Delay 3.0)
  (bind _asbp_game_instance (Utilities|Casting|CastToBP_GameInstance (Game|GetGameInstance)))
  (Variables|/Game/Jaehak/GameInstance/BP_GameInstance.BP_GameInstance_C|SetTeleportationTag _asbp_game_instance (Variables|Default|GetTeleTag))
  (Game|OpenLevel(byName) (Variables|Default|GetDestination%20Tag)))

(event EventBeginPlay
  (bind _asbp_interaction_ui (Utilities|Casting|CastToBP_Interaction_UI (UserInterface|GetUserWidgetObject (Variables|Default|GetWidget))))
  (Variables|/Game/Jaehak/Widget/BP_Interaction_UI.BP_Interaction_UI_C|SetNameValue _asbp_interaction_ui (Utilities|Text|ToText(String) (Variables|Default|GetGameName))))

(event Collision|EventActorBeginOverlap
  (params (OtherActor :type Actor%20Object%20Reference)))

(event EventTick
  (params (DeltaSeconds :type Float%20%28single-precision%29)))

(fn ConstructionScript)