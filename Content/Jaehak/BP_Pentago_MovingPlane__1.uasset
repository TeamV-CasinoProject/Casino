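; Actor for a moving board plane in a Pentago game that animates a slide, rotate and slide-back move.
; On BeginPlay it creates the Pentago_UI1 widget and binds its P1R1 and P1R2 dispatchers to matching events.
; Each event waits, then runs move, yaw-rotation and move-back timelines, with P1R2 negating the yaw.
; Stages chain through Delays on each timeline's Update output rather than Finished.
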(event Custom|P1%20R1
  (Utilities|FlowControl|Delay 2.0)
  (bind _move_location (Timeline|Timeline Play)
    (:Update
      (Transformation|SetActorLocation _move_location false false)
      (Utilities|FlowControl|Delay 1.5)
      (bind _rotate_value (Timeline|Timeline_0 Play)
        (:Update
          (Transformation|SetActorRotation (Math|Rotator|MakeRotator 0.0 0.0 _rotate_value))
          (Utilities|FlowControl|Delay 1.5)
          (bind _move_location_2 (Timeline|Timeline_1 Play)
            (:Update
              (Transformation|SetActorLocation _move_location_2 false false))))))))

(event Custom|P1%20R2
  (Utilities|FlowControl|Delay 2.0)
  (bind _move_location (Timeline|Move_Timline Play)
    (:Update
      (Transformation|SetActorLocation _move_location false false)
      (Utilities|FlowControl|Delay 1.5)
      (bind _rotate_value (Timeline|Rotate_Timeline Play)
        (:Update
          (Transformation|SetActorRotation (Math|Rotator|MakeRotator 0.0 0.0 (* _rotate_value -1.0)))
          (Utilities|FlowControl|Delay 1.5)
          (bind _move_location_2 (Timeline|MoveBack_Timeline Play)
            (:Update
              (Transformation|SetActorLocation _move_location_2 false false))))))))

(event EventBeginPlay
  (bind _returnvalue (UserInterface|CreateWidget "/Game/Jaehak/Pentago_UI1.Pentago_UI1_C"))
  (UserInterface|Viewport|AddtoViewport _returnvalue 0)
  (EventDispatchers|BindEventtoP1R1Dispatcher _returnvalue (delegate Custom|P1%20R1))
  (EventDispatchers|BindEventtoP1R2Dispatcher _returnvalue (delegate Custom|P1%20R2)))

(fn ConstructionScript)