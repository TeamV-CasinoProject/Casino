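; Test actor that moves its Cube component between the MovingPoint and BackPoint references on BeginPlay.
; Timed MoveComponentTo calls and delays send it to MovingPoint, apply a 90-degree rotation, then move it to BackPoint, passing world locations as relative targets.
; A hard-wired true branch leaves the opposite-rotation path unused.
; Disconnected nodes hold unused experiments with local actor transforms and component attachment.
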(event EventBeginPlay
  (bind _movingpoint (Variables|Default|GetMovingPoint))
  (bind _backpoint (Variables|Default|GetBackPoint))
  (bind _cube (Variables|Default|GetCube))
  (bind _cube_2 (Variables|Default|GetCube))
  (bind _returnvalue (Transformation|GetActorLocation _movingpoint))
  (bind _returnvalue_2 (Transformation|GetActorLocation _backpoint))
  (Components|MoveComponentTo (Variables|Default|GetCube) _returnvalue "0, 0, 0" false false 1.0 false)
  (Utilities|FlowControl|Delay 1.0)
  (if true
    (Components|MoveComponentTo _cube _returnvalue "0.000000,90.000000,0.000000" false false 1.5 false)
    (Utilities|FlowControl|Delay 1.0)
    (Components|MoveComponentTo _cube _returnvalue_2 "0.000000,90.000000,0.000000" false false 1.5 false)
    (else
      (Components|MoveComponentTo _cube_2 _returnvalue "0.000000,-90.000000,0.000000" false false 1.5 false)
      (Utilities|FlowControl|Delay 1.0)
      (Components|MoveComponentTo _cube_2 _returnvalue_2 "0, 0, 0" false false 1.5 false))))

(fn ConstructionScript)