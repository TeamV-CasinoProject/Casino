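; Rotating board quadrant 4 of a Pentago game, turned 90 degrees either way by events bound to BP_RotationUI.
; Each turn snapshots nine SlotChecker values and permutes them around the fixed centre.
; MoveComponentTo then slides the plane to MovePoint, yaws it and returns it to BackPoint, before BPWinChecker is updated and TurnValue flips.
; An older teleport-based version (P4R1/P4R2) and stepped movement macros remain, with their hookups disconnected.
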(event Custom|P4C%20RC
  (bind _bp_winchecker (Variables|Default|GetBP_WinChecker))
  (bind _staticmeshcomponent (Variables|Debug|GetStaticMeshComponent))
  (bind _movepoint (Variables|Default|GetMovePoint))
  (bind _returnvalue (Transformation|GetActorLocation _movepoint))
  (Utilities|FlowControl|Delay 1.0)
  (CallFunction|SlotValueSetting)
  (CallFunction|RClockRotation)
  (Components|MoveComponentTo _staticmeshcomponent _returnvalue (Variables|Default|GetCurrentRotator) false false 0.35 false)
  (Utilities|FlowControl|Delay 0.15)
  (Components|MoveComponentTo _staticmeshcomponent _returnvalue (Math|Rotator|MakeRotator (.Roll (Math|Rotator|BreakRotator (Variables|Default|GetCurrentRotator))) (.Pitch (Math|Rotator|BreakRotator (Variables|Default|GetCurrentRotator))) (- (.Yaw (Math|Rotator|BreakRotator (Variables|Default|GetCurrentRotator))) 9e+01)) false false 0.25 false)
  (Utilities|FlowControl|Delay 0.15)
  (Components|MoveComponentTo _staticmeshcomponent (Transformation|GetActorLocation (Variables|Default|GetBackPoint)) (Math|Rotator|MakeRotator (.Roll (Math|Rotator|BreakRotator (Variables|Default|GetCurrentRotator))) (.Pitch (Math|Rotator|BreakRotator (Variables|Default|GetCurrentRotator))) (- (.Yaw (Math|Rotator|BreakRotator (Variables|Default|GetCurrentRotator))) 9e+01)) false false 0.35 false)
  (Variables|Default|SetCurrentRotator (Math|Rotator|MakeRotator (.Roll (Math|Rotator|BreakRotator (Variables|Default|GetCurrentRotator))) (.Pitch (Math|Rotator|BreakRotator (Variables|Default|GetCurrentRotator))) (- (.Yaw (Math|Rotator|BreakRotator (Variables|Default|GetCurrentRotator))) 9e+01)))
  (Default|CallRotationUpdateP41 (Variables|Default|GetBP_WinChecker))
  (if (Variables|/Game/Jaehak/BP_WinChecker.BP_WinChecker_C|GetTurnValue _bp_winchecker)
    (Variables|/Game/Jaehak/BP_WinChecker.BP_WinChecker_C|SetTurnValue _bp_winchecker false)
    (else
      (Variables|/Game/Jaehak/BP_WinChecker.BP_WinChecker_C|SetTurnValue _bp_winchecker true))))

(event Custom|P4R%20C
  (bind _bp_winchecker (Variables|Default|GetBP_WinChecker))
  (bind _staticmeshcomponent (Variables|Debug|GetStaticMeshComponent))
  (bind _movepoint (Variables|Default|GetMovePoint))
  (bind _returnvalue (Transformation|GetActorLocation _movepoint))
  (Utilities|FlowControl|Delay 1.0)
  (CallFunction|SlotValueSetting)
  (CallFunction|ClockRotation)
  (Components|MoveComponentTo _staticmeshcomponent _returnvalue (Variables|Default|GetCurrentRotator) false false 0.35 false)
  (Utilities|FlowControl|Delay 0.15)
  (Components|MoveComponentTo _staticmeshcomponent _returnvalue (Math|Rotator|MakeRotator (.Roll (Math|Rotator|BreakRotator (Variables|Default|GetCurrentRotator))) (.Pitch (Math|Rotator|BreakRotator (Variables|Default|GetCurrentRotator))) (+ (.Yaw (Math|Rotator|BreakRotator (Variables|Default|GetCurrentRotator))) 9e+01)) false false 0.25 false)
  (Utilities|FlowControl|Delay 0.15)
  (Components|MoveComponentTo _staticmeshcomponent (Transformation|GetActorLocation (Variables|Default|GetBackPoint)) (Math|Rotator|MakeRotator (.Roll (Math|Rotator|BreakRotator (Variables|Default|GetCurrentRotator))) (.Pitch (Math|Rotator|BreakRotator (Variables|Default|GetCurrentRotator))) (+ (.Yaw (Math|Rotator|BreakRotator (Variables|Default|GetCurrentRotator))) 9e+01)) false false 0.35 false)
  (Variables|Default|SetCurrentRotator (Math|Rotator|MakeRotator (.Roll (Math|Rotator|BreakRotator (Variables|Default|GetCurrentRotator))) (.Pitch (Math|Rotator|BreakRotator (Variables|Default|GetCurrentRotator))) (+ (.Yaw (Math|Rotator|BreakRotator (Variables|Default|GetCurrentRotator))) 9e+01)))
  (Default|CallRotationUpdateP42 (Variables|Default|GetBP_WinChecker))
  (if (Variables|/Game/Jaehak/BP_WinChecker.BP_WinChecker_C|GetTurnValue _bp_winchecker)
    (Variables|/Game/Jaehak/BP_WinChecker.BP_WinChecker_C|SetTurnValue _bp_winchecker false)
    (else
      (Variables|/Game/Jaehak/BP_WinChecker.BP_WinChecker_C|SetTurnValue _bp_winchecker true))))

(event Custom|P4%20R2
  (bind _bp_winchecker (Variables|Default|GetBP_WinChecker))
  (Development|PrintString "C")
  (Utilities|FlowControl|Delay 2.0)
  (CallFunction|SlotValueSetting)
  (CallFunction|ClockRotation)
  (Transformation|SetActorLocation (Transformation|GetActorLocation (Variables|Default|GetMovePoint)) false false)
  (Utilities|FlowControl|Delay 1.5)
  (Transformation|SetActorRotation (.90 (|RoationValue)))
  (Utilities|FlowControl|Delay 1.5)
  (Transformation|SetActorLocation (Transformation|GetActorLocation (Variables|Default|GetBackPoint)) false false)
  (Default|CallRotationUpdateP42 (Variables|Default|GetBP_WinChecker))
  (Development|PrintString "_____________________")
  (if (Variables|/Game/Jaehak/BP_WinChecker.BP_WinChecker_C|GetTurnValue _bp_winchecker)
    (Variables|/Game/Jaehak/BP_WinChecker.BP_WinChecker_C|SetTurnValue _bp_winchecker false)
    (Development|PrintString "PtoA")
    (else
      (Variables|/Game/Jaehak/BP_WinChecker.BP_WinChecker_C|SetTurnValue _bp_winchecker true)
      (Development|PrintString "AtoP"))))

(event Custom|P4%20R1
  (bind _bp_winchecker (Variables|Default|GetBP_WinChecker))
  (Development|PrintString "RC")
  (Utilities|FlowControl|Delay 2.0)
  (CallFunction|SlotValueSetting)
  (CallFunction|RClockRotation)
  (Transformation|SetActorLocation (Transformation|GetActorLocation (Variables|Default|GetMovePoint)) false false)
  (Utilities|FlowControl|Delay 1.5)
  (Transformation|SetActorRotation (.-90 (|RoationValue)))
  (Utilities|FlowControl|Delay 1.5)
  (Transformation|SetActorLocation (Transformation|GetActorLocation (Variables|Default|GetBackPoint)) false false)
  (Default|CallRotationUpdateP41 (Variables|Default|GetBP_WinChecker))
  (Development|PrintString "_____________________")
  (if (Variables|/Game/Jaehak/BP_WinChecker.BP_WinChecker_C|GetTurnValue _bp_winchecker)
    (Variables|/Game/Jaehak/BP_WinChecker.BP_WinChecker_C|SetTurnValue _bp_winchecker false)
    (Development|PrintString "PtoA")
    (else
      (Variables|/Game/Jaehak/BP_WinChecker.BP_WinChecker_C|SetTurnValue _bp_winchecker true)
      (Development|PrintString "AtoP"))))

(event EventBeginPlay
  (CallFunction|SlotValueSetting)
  (bind _foundwidgets (Widget|GetAllWidgetsOfClass "/Game/Jaehak/Widget/BP_RotationUI.BP_RotationUI_C" true))
  (EventDispatchers|BindEventtoP4RRCEvent (Utilities|Array|Get(acopy) _foundwidgets) (delegate Custom|P4C%20RC))
  (EventDispatchers|BindEventtoP4RCEvent (Utilities|Array|Get(acopy) _foundwidgets) (delegate Custom|P4R%20C))
  (Variables|Default|SetCurrentRotator (Transformation|GetActorRotation)))

(fn ConstructionScript)

(fn RClockRotation
  (bind _slotvaluearray (Variables|Default|GetSlotValueArray))
  (Variables|/Game/Jaehak/AI/BP_Pentago_Checker.BP_Pentago_Checker_C|Setslot_Value (Variables|Default|GetSlotChecker1) (Utilities|Array|Get(acopy) _slotvaluearray 2))
  (Variables|/Game/Jaehak/AI/BP_Pentago_Checker.BP_Pentago_Checker_C|Setslot_Value (Variables|Default|GetSlotChecker2) (Utilities|Array|Get(acopy) _slotvaluearray 5))
  (Variables|/Game/Jaehak/AI/BP_Pentago_Checker.BP_Pentago_Checker_C|Setslot_Value (Variables|Default|GetSlotChecker3) (Utilities|Array|Get(acopy) _slotvaluearray 8))
  (Variables|/Game/Jaehak/AI/BP_Pentago_Checker.BP_Pentago_Checker_C|Setslot_Value (Variables|Default|GetSlotChecker4) (Utilities|Array|Get(acopy) _slotvaluearray 1))
  (Variables|/Game/Jaehak/AI/BP_Pentago_Checker.BP_Pentago_Checker_C|Setslot_Value (Variables|Default|GetSlotChecker6) (Utilities|Array|Get(acopy) _slotvaluearray 7))
  (Variables|/Game/Jaehak/AI/BP_Pentago_Checker.BP_Pentago_Checker_C|Setslot_Value (Variables|Default|GetSlotChecker7) (Utilities|Array|Get(acopy) _slotvaluearray))
  (Variables|/Game/Jaehak/AI/BP_Pentago_Checker.BP_Pentago_Checker_C|Setslot_Value (Variables|Default|GetSlotChecker8) (Utilities|Array|Get(acopy) _slotvaluearray 3))
  (Variables|/Game/Jaehak/AI/BP_Pentago_Checker.BP_Pentago_Checker_C|Setslot_Value (Variables|Default|GetSlotChecker9) (Utilities|Array|Get(acopy) _slotvaluearray 6)))

(fn SlotValueSetting
  (Variables|Default|SetSlotValueArray (Utilities|Array|MakeArray (Variables|/Game/Jaehak/AI/BP_Pentago_Checker.BP_Pentago_Checker_C|Getslot_Value (Variables|Default|GetSlotChecker1)) (Variables|/Game/Jaehak/AI/BP_Pentago_Checker.BP_Pentago_Checker_C|Getslot_Value (Variables|Default|GetSlotChecker2)) (Variables|/Game/Jaehak/AI/BP_Pentago_Checker.BP_Pentago_Checker_C|Getslot_Value (Variables|Default|GetSlotChecker3)) (Variables|/Game/Jaehak/AI/BP_Pentago_Checker.BP_Pentago_Checker_C|Getslot_Value (Variables|Default|GetSlotChecker4)) (Variables|/Game/Jaehak/AI/BP_Pentago_Checker.BP_Pentago_Checker_C|Getslot_Value (Variables|Default|GetSlotChecker5)) (Variables|/Game/Jaehak/AI/BP_Pentago_Checker.BP_Pentago_Checker_C|Getslot_Value (Variables|Default|GetSlotChecker6)) (Variables|/Game/Jaehak/AI/BP_Pentago_Checker.BP_Pentago_Checker_C|Getslot_Value (Variables|Default|GetSlotChecker7)) (Variables|/Game/Jaehak/AI/BP_Pentago_Checker.BP_Pentago_Checker_C|Getslot_Value (Variables|Default|GetSlotChecker8)) (Variables|/Game/Jaehak/AI/BP_Pentago_Checker.BP_Pentago_Checker_C|Getslot_Value (Variables|Default|GetSlotChecker9)))))

(fn ClockRotation
  (bind _slotvaluearray (Variables|Default|GetSlotValueArray))
  (Variables|/Game/Jaehak/AI/BP_Pentago_Checker.BP_Pentago_Checker_C|Setslot_Value (Variables|Default|GetSlotChecker1) (Utilities|Array|Get(acopy) _slotvaluearray 6))
  (Variables|/Game/Jaehak/AI/BP_Pentago_Checker.BP_Pentago_Checker_C|Setslot_Value (Variables|Default|GetSlotChecker2) (Utilities|Array|Get(acopy) _slotvaluearray 3))
  (Variables|/Game/Jaehak/AI/BP_Pentago_Checker.BP_Pentago_Checker_C|Setslot_Value (Variables|Default|GetSlotChecker3) (Utilities|Array|Get(acopy) _slotvaluearray))
  (Variables|/Game/Jaehak/AI/BP_Pentago_Checker.BP_Pentago_Checker_C|Setslot_Value (Variables|Default|GetSlotChecker4) (Utilities|Array|Get(acopy) _slotvaluearray 7))
  (Variables|/Game/Jaehak/AI/BP_Pentago_Checker.BP_Pentago_Checker_C|Setslot_Value (Variables|Default|GetSlotChecker6) (Utilities|Array|Get(acopy) _slotvaluearray 1))
  (Variables|/Game/Jaehak/AI/BP_Pentago_Checker.BP_Pentago_Checker_C|Setslot_Value (Variables|Default|GetSlotChecker7) (Utilities|Array|Get(acopy) _slotvaluearray 8))
  (Variables|/Game/Jaehak/AI/BP_Pentago_Checker.BP_Pentago_Checker_C|Setslot_Value (Variables|Default|GetSlotChecker8) (Utilities|Array|Get(acopy) _slotvaluearray 5))
  (Variables|/Game/Jaehak/AI/BP_Pentago_Checker.BP_Pentago_Checker_C|Setslot_Value (Variables|Default|GetSlotChecker9) (Utilities|Array|Get(acopy) _slotvaluearray 2)))