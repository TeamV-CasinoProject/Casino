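; Moving board plane for a Pentago game, apparently one quadrant, that animates a move, twist and return after a two-second delay at BeginPlay.
; Three timelines drive absolute location, yaw and return location, with the constant-false branch always negating the yaw.
; Each next timeline starts through a Delay on the previous one's Update output rather than Finished, so stages can overlap.
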(event EventBeginPlay
  (Utilities|FlowControl|Delay 2.0)
  (bind _move_location (Timeline|Move_Timline Play)
    (:Update
      (Transformation|SetActorLocation _move_location false false)
      (Utilities|FlowControl|Delay 1.5)
      (bind _rotate_value (Timeline|Rotate_Timeline Play)
        (:Update
          (if false
            (Transformation|SetActorRotation (Math|Rotator|MakeRotator 0.0 0.0 _rotate_value))
            (else
              (Transformation|SetActorRotation (Math|Rotator|MakeRotator 0.0 0.0 (* _rotate_value -1.0)))))
          (Utilities|FlowControl|Delay 1.5)
          (bind _move_location_2 (Timeline|MoveBack_Timeline Play)
            (:Update
              (Transformation|SetActorLocation _move_location_2 false false))))))))

(fn ConstructionScript)