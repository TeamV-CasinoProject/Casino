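; Pentago plane actor that runs a one-time scripted move and turn of a board plane at BeginPlay.
; It finds the first actor of PentagoPlane's class, which may differ from the referenced instance, and waits a configurable delay.
; A single VInterpTo call, not a per-tick interpolation, sets that actor's location toward MovingPoint.
; After another pause, it applies a fixed local rotation to that actor's root component.
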(event EventBeginPlay
  (bind _pentago_plane (Variables|Default|GetPentago_Plane))
  (Development|PrintString (Utilities|GetDisplayName _pentago_plane))
  (bind _returnvalue (Actor|GetActorOfClass (Utilities|GetClass _pentago_plane)))
  (Utilities|FlowControl|Delay (Variables|Default|GetDelay_Time))
  (Transformation|SetActorLocation _returnvalue (Math|Interpolation|VInterpTo (Transformation|GetActorLocation (Variables|Default|GetPentago_Plane)) (Transformation|GetActorLocation (Variables|Default|GetMoving_Point)) 5.0 0.0) false false)
  (Utilities|FlowControl|Delay 2.0)
  (Transformation|AddLocalRotation (Variables|/Script/Engine.Actor|GetRootComponent _returnvalue) "0.000000,60.000000,0.000000" false false))

(fn ConstructionScript)