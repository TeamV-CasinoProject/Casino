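; Pentago plane Blueprint that slides its static mesh once after a delay at the start of play.
; BeginPlay prints the PentagoPlane's name, looks up an actor of that class, waits DelayTime, then eases the mesh to a fixed relative offset with MoveComponentTo.
; Tick is empty, and the interpolation logic for moving toward MovingPoint and rotating is disconnected, so it never runs.
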(event EventTick
  (params (DeltaSeconds :type Float%20%28single-precision%29)))

(event EventBeginPlay
  (bind _pentago_plane (Variables|Default|GetPentago_Plane))
  (Development|PrintString (Utilities|GetDisplayName _pentago_plane))
  (bind _returnvalue (Actor|GetActorOfClass (Utilities|GetClass _pentago_plane)))
  (Utilities|FlowControl|Delay (Variables|Default|GetDelay_Time))
  (Components|MoveComponentTo (Variables|Debug|GetStaticMeshComponent) "-100.000000,0.000000,0.000000" "0, 0, 0" true true 5.0 false))

(fn ConstructionScript)