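; Movable third quadrant of a Pentago board, rotated when its BP_Pentago_UI3 widget fires a P3R1 or P3R2 dispatcher.
; Each event snapshots nine SlotChecker values and permutes them clockwise or counter-clockwise around the fixed center.
; The plane jumps to MovePoint, rotates and returns with delays between steps, both events using the same RoationValue output.
; BPWinChecker then gets the rotation update and its turn flag flips; timeline-based animation is left unconnected.
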(event Custom|P3R2
  (bind _bp_winchecker (Variables|Default|GetBP_WinChecker))
  (Development|PrintString "C")
  (Utilities|FlowControl|Delay 2.0)
  (CallFunction|SlotValueSetting)
  (CallFunction|ClockRotation)
  (Transformation|SetActorLocation (Transformation|GetActorLocation (Variables|Default|GetMovePoint)) false false)
  (Utilities|FlowControl|Delay 1.5)
  (Transformation|SetActorRotation (.90 (|RoationValue)))
  (Utilities|FlowControl|Delay 1.5)
  (Transformation|SetActorLocation (Transformation|GetActorLocation (Variables|Default|GetBackPojnt)) false false)
  (Default|CallRotationUpdateP32 (Variables|Default|GetBP_WinChecker))
  (Development|PrintString "_____________________")
  (if (Variables|/Game/Jaehak/BP_WinChecker.BP_WinChecker_C|GetTurnValue _bp_winchecker)
    (Variables|/Game/Jaehak/BP_WinChecker.BP_WinChecker_C|SetTurnValue _bp_winchecker false)
    (Development|PrintString "PtoA")
    (else
      (Variables|/Game/Jaehak/BP_WinChecker.BP_WinChecker_C|SetTurnValue _bp_winchecker true)
      (Development|PrintString "AtoP"))))

(event Custom|R3%20R1
  (bind _bp_winchecker (Variables|Default|GetBP_WinChecker))
  (Development|PrintString "RC")
  (Utilities|FlowControl|Delay 2.0)
  (CallFunction|SlotValueSetting)
  (CallFunction|RClockRotation)
  (Transformation|SetActorLocation (Transformation|GetActorLocation (Variables|Default|GetMovePoint)) false false)
  (Utilities|FlowControl|Delay 1.5)
  (Transformation|SetActorRotation (.-90 (|RoationValue)))
  (Utilities|FlowControl|Delay 1.5)
  (Transformation|SetActorLocation (Transformation|GetActorLocation (Variables|Default|GetBackPojnt)) false false)
  (Default|CallRotationUpdateP31 (Variables|Default|GetBP_WinChecker))
  (Development|PrintString "_____________________")
  (if (Variables|/Game/Jaehak/BP_WinChecker.BP_WinChecker_C|GetTurnValue _bp_winchecker)
    (Variables|/Game/Jaehak/BP_WinChecker.BP_WinChecker_C|SetTurnValue _bp_winchecker false)
    (Development|PrintString "PtoA")
    (else
      (Variables|/Game/Jaehak/BP_WinChecker.BP_WinChecker_C|SetTurnValue _bp_winchecker true)
      (Development|PrintString "AtoP"))))

(event EventBeginPlay
  (CallFunction|SlotValueSetting)
  (bind _returnvalue (UserInterface|CreateWidget "/Game/Jaehak/Widget/BP_Pentago_UI3.BP_Pentago_UI3_C"))
  (UserInterface|Viewport|AddtoViewport _returnvalue 0)
  (EventDispatchers|BindEventtoP3R1Dispatcher _returnvalue (delegate Custom|R3%20R1))
  (EventDispatchers|BindEventtoP3R2Dispatcher _returnvalue (delegate Custom|P3R2)))

(fn ConstructionScript)

(fn HandleButtonClick)

(fn SlotValueSetting
  (Variables|Default|SetSlotValueArray (Utilities|Array|MakeArray (Variables|/Game/Jaehak/BP_Pentago_Checker.BP_Pentago_Checker_C|Getslot_Value (Variables|Default|GetSlotChecker1)) (Variables|/Game/Jaehak/BP_Pentago_Checker.BP_Pentago_Checker_C|Getslot_Value (Variables|Default|GetSlotChecker2)) (Variables|/Game/Jaehak/BP_Pentago_Checker.BP_Pentago_Checker_C|Getslot_Value (Variables|Default|GetSlotChecker3)) (Variables|/Game/Jaehak/BP_Pentago_Checker.BP_Pentago_Checker_C|Getslot_Value (Variables|Default|GetSlotChecker4)) (Variables|/Game/Jaehak/BP_Pentago_Checker.BP_Pentago_Checker_C|Getslot_Value (Variables|Default|GetSlotChecker5)) (Variables|/Game/Jaehak/BP_Pentago_Checker.BP_Pentago_Checker_C|Getslot_Value (Variables|Default|GetSlotChecker6)) (Variables|/Game/Jaehak/BP_Pentago_Checker.BP_Pentago_Checker_C|Getslot_Value (Variables|Default|GetSlotChecker7)) (Variables|/Game/Jaehak/BP_Pentago_Checker.BP_Pentago_Checker_C|Getslot_Value (Variables|Default|GetSlotChecker8)) (Variables|/Game/Jaehak/BP_Pentago_Checker.BP_Pentago_Checker_C|Getslot_Value (Variables|Default|GetSlotChecker9))))
  (Development|PrintString "SlotValueSetting"))

(fn RClockRotation
  (bind _slotvaluearray (Variables|Default|GetSlotValueArray))
  (Development|PrintString "changeValue")
  (Variables|/Game/Jaehak/BP_Pentago_Checker.BP_Pentago_Checker_C|Setslot_Value (Variables|Default|GetSlotChecker1) (Utilities|Array|Get(acopy) _slotvaluearray 2))
  (Variables|/Game/Jaehak/BP_Pentago_Checker.BP_Pentago_Checker_C|Setslot_Value (Variables|Default|GetSlotChecker2) (Utilities|Array|Get(acopy) _slotvaluearray 5))
  (Variables|/Game/Jaehak/BP_Pentago_Checker.BP_Pentago_Checker_C|Setslot_Value (Variables|Default|GetSlotChecker3) (Utilities|Array|Get(acopy) _slotvaluearray 8))
  (Variables|/Game/Jaehak/BP_Pentago_Checker.BP_Pentago_Checker_C|Setslot_Value (Variables|Default|GetSlotChecker4) (Utilities|Array|Get(acopy) _slotvaluearray 1))
  (Variables|/Game/Jaehak/BP_Pentago_Checker.BP_Pentago_Checker_C|Setslot_Value (Variables|Default|GetSlotChecker6) (Utilities|Array|Get(acopy) _slotvaluearray 7))
  (Variables|/Game/Jaehak/BP_Pentago_Checker.BP_Pentago_Checker_C|Setslot_Value (Variables|Default|GetSlotChecker7) (Utilities|Array|Get(acopy) _slotvaluearray))
  (Variables|/Game/Jaehak/BP_Pentago_Checker.BP_Pentago_Checker_C|Setslot_Value (Variables|Default|GetSlotChecker8) (Utilities|Array|Get(acopy) _slotvaluearray 3))
  (Variables|/Game/Jaehak/BP_Pentago_Checker.BP_Pentago_Checker_C|Setslot_Value (Variables|Default|GetSlotChecker9) (Utilities|Array|Get(acopy) _slotvaluearray 6)))

(fn ClockRotation
  (bind _slotvaluearray (Variables|Default|GetSlotValueArray))
  (Variables|/Game/Jaehak/BP_Pentago_Checker.BP_Pentago_Checker_C|Setslot_Value (Variables|Default|GetSlotChecker1) (Utilities|Array|Get(acopy) _slotvaluearray 6))
  (Variables|/Game/Jaehak/BP_Pentago_Checker.BP_Pentago_Checker_C|Setslot_Value (Variables|Default|GetSlotChecker2) (Utilities|Array|Get(acopy) _slotvaluearray 3))
  (Variables|/Game/Jaehak/BP_Pentago_Checker.BP_Pentago_Checker_C|Setslot_Value (Variables|Default|GetSlotChecker3) (Utilities|Array|Get(acopy) _slotvaluearray))
  (Variables|/Game/Jaehak/BP_Pentago_Checker.BP_Pentago_Checker_C|Setslot_Value (Variables|Default|GetSlotChecker4) (Utilities|Array|Get(acopy) _slotvaluearray 7))
  (Variables|/Game/Jaehak/BP_Pentago_Checker.BP_Pentago_Checker_C|Setslot_Value (Variables|Default|GetSlotChecker6) (Utilities|Array|Get(acopy) _slotvaluearray 1))
  (Variables|/Game/Jaehak/BP_Pentago_Checker.BP_Pentago_Checker_C|Setslot_Value (Variables|Default|GetSlotChecker7) (Utilities|Array|Get(acopy) _slotvaluearray 8))
  (Variables|/Game/Jaehak/BP_Pentago_Checker.BP_Pentago_Checker_C|Setslot_Value (Variables|Default|GetSlotChecker8) (Utilities|Array|Get(acopy) _slotvaluearray 5))
  (Variables|/Game/Jaehak/BP_Pentago_Checker.BP_Pentago_Checker_C|Setslot_Value (Variables|Default|GetSlotChecker9) (Utilities|Array|Get(acopy) _slotvaluearray 2)))