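; BP_Stone_Spawner is a clickable board spot that places a black or white Pentago stone for the current turn.
; On click it reads TurnValue on BPWinChecker, then spawns the matching stone and attaches it to itself.
; It fires the matching spawn event on Checker, flips the turn and calls the win checker's click event check.
; Nothing in the click handler guards against repeat clicks.
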(event Collision|EventActorBeginOverlap
  (params (OtherActor :type Actor%20Object%20Reference)))

(event EventTick
  (params (DeltaSeconds :type Float%20%28single-precision%29)))

(event MouseInput|EventActorOnClicked
  (params (ButtonPressed :type Key%20Structure :default "None"))
  (bind _returnvalue (Math|Conversions|ToTransform(Vector) "0, 0, 0"))
  (bind _self self)
  (bind _bp_winchecker (Variables|Default|GetBP_WinChecker))
  (bind _checker (Variables|Default|GetChecker))
  (if (Variables|/Game/Jaehak/BP_WinChecker.BP_WinChecker_C|GetTurnValue (Variables|Default|GetBP_WinChecker))
    (bind _returnvalue_2 (Game|SpawnActorfromClass "/Game/Jaehak/BP_Pentago_Stone_Black.BP_Pentago_Stone_Black_C" _returnvalue "Undefined" "MultiplyWithRoot" 0 0))
    (Transformation|AttachActorToActor _returnvalue_2 _self "None" "KeepRelative" "KeepRelative" "KeepRelative" true)
    (Default|CallSpawnBlackEvent _checker)
    (Variables|/Game/Jaehak/BP_WinChecker.BP_WinChecker_C|SetTurnValue _bp_winchecker false)
    (else
      (bind _returnvalue_3 (Game|SpawnActorfromClass "/Game/Jaehak/BP_Pentago_Stone_White.BP_Pentago_Stone_White_C" _returnvalue "Undefined" "MultiplyWithRoot" 0 0))
      (Transformation|AttachActorToActor _returnvalue_3 _self "None" "KeepRelative" "KeepRelative" "KeepRelative" true)
      (Default|CallSpawnWhiteEvent _checker)
      (Variables|/Game/Jaehak/BP_WinChecker.BP_WinChecker_C|SetTurnValue _bp_winchecker true)))
  (Default|CallClickEventCheck _bp_winchecker))

(event EventBeginPlay)

(fn ConstructionScript)